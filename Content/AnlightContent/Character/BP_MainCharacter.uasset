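; Main character Blueprint that hooks up health, stamina and sprint components, with debug feedback for testing them.
; Health and stamina change and depletion events print on-screen messages, and the K and M keys lower and raise health.
; The sprint input action calls StartSprint on the sprint component, with no stop call in this graph.
; A stamina decrease node is left unconnected and never runs.
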(event `self.HealthComponent.OnHealthChanged`
  (params (NewHealth :type "Float (single-precision)") (maxHealth :type "Float (single-precision)"))
  (`KismetSystemLibrary.PrintString` (`KismetTextLibrary.Conv_TextToString` (`|FormatText` "Health: {Health} / {MaxHealth}" NewHealth maxHealth)) true true (struct :`R` 0.052679 :`G` 1.0 :`B` 0.0032 :`A` 1.0)))

(event `self.HealthComponent.OnHealthDepleted`
  (`KismetSystemLibrary.PrintString` "You dead <3" true true (struct :`R` 1.0 :`G` 0.061935 :`A` 1.0)))

(event `Key|K`
  (params (Key :type "Key Structure"))
  (:`Pressed`
    (`HealthComponent.UpdateHealth` (`self.HealthComponent`) -10.0)))

(event `Key|M`
  (params (Key :type "Key Structure"))
  (:`Pressed`
    (`HealthComponent.UpdateHealth` (`self.HealthComponent`) 10.0)))

(event `self.StaminaComponent.OnStaminaChanged`
  (params (NewStamina :type "Float (single-precision)") (MaxStamina :type "Float (single-precision)"))
  (`KismetSystemLibrary.PrintString` (`KismetTextLibrary.Conv_TextToString` (`|FormatText` "Stamina: {Stamina} / {MaxStamina}" NewStamina MaxStamina))))

(event `self.StaminaComponent.OnStaminaDepleted`
  (`KismetSystemLibrary.PrintString` "Stamina is empty" true true (struct :`R` 1.0 :`G` 0.795137 :`A` 1.0)))

(event `EnhancedInput|/Game/AnlightContent/Character/A_Actions/A-IA_Sprint`
  (params (ActionValue :type Boolean) (ElapsedSeconds :type "Float (double-precision)") (TriggeredSeconds :type "Float (double-precision)") (InputAction :type "InputAction Object Reference" :default "/Game/AnlightContent/Character/A_Actions/A-IA_Sprint.A-IA_Sprint"))
  (:`Triggered`
    (`SprintComponent.StartSprint` (`self.SprintComponent`))))

(fn `UserConstructionScript`)